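; BP_Door is a locked door that responds to a character carrying a matching key.
; Its Interact event scans the character's InventoryArray for a BP_Key with the same KeyID and calls DoorClickedWithKey on a match.
; DoorFunc toggles DoorOpen and snaps the actor between two hardcoded locations and rotations without sweep.
; Nothing in this Blueprint calls DoorFunc directly.
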(event EventInteract
  (params (Character :type My%20Character%20Object%20Reference))
  ;[1 1 1] Check if BP_Character has Key, if yes = do smth.
  (bind _array_element (Utilities|Array|ForEachLoopwithBreak (Variables|/Game/Blueprints/MyCharacter.MyCharacter_C|GetInventory%20Array Character))
    (:LoopBody
      (bind _asbp_key (Utilities|Casting|CastToBP_Key _array_element))
      (if (== (Variables|/Game/Assets/Blueprints/BP_Key.BP_Key_C|GetKeyID _asbp_key) (Variables|Default|GetKeyID))
        (Default|CallDoorClickedwithKey)))))

(fn ConstructionScript)

(fn DoorFunc
  (if (Variables|Default|GetDoorOpen)
    (Transformation|SetActorLocation "-375.000000,733.000000, 0" false)
    (Transformation|SetActorRotation "0.000000,-90.000000,0.000000")
    (Variables|Default|SetDoorOpen false)
    (else
      (Transformation|SetActorLocation "-427.000000,782.000000, 0" false)
      (Transformation|SetActorRotation "0.000000,-168.000000,0.000000")
      (Variables|Default|SetDoorOpen true))))